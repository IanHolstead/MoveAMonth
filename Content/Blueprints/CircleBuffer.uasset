(fn CreateFloatBuffer
  (params (size :type Integer))
  (Utilities|Array|Resize (LocalVariables|Getarray) size)
  (return (LocalVariables|Getarray)))

(fn SetItemFloatBuffer
  (params (buffer :type Array%20of%20Floats%20%28single-precision%29) (index :type Integer) (item :type Float%20%28single-precision%29))
  (bind _returnvalue (Utilities|Array|Length buffer))
  (bind _returnvalue_2 (Math|Integer|%(Integer) index _returnvalue))
  (LocalVariables|Setchanged (Utilities|Array|Get(acopy) buffer _returnvalue_2))
  (Utilities|Array|SetArrayElem buffer _returnvalue_2 item)
  (return (LocalVariables|Getchanged)))

(fn SetItemVectorBuffer
  (params (buffer :type Array%20of%20Vectors) (index :type Integer) (item :type Vector))
  (bind _returnvalue (Utilities|Array|Length buffer))
  (bind _returnvalue_2 (Math|Integer|%(Integer) index _returnvalue))
  (LocalVariables|Setchanged (Utilities|Array|Get(acopy) buffer _returnvalue_2))
  (Utilities|Array|SetArrayElem buffer _returnvalue_2 item)
  (return (LocalVariables|Getchanged)))

(fn CreateVectorBuffer
  (params (size :type Integer))
  (Utilities|Array|Resize (LocalVariables|Getarray) size)
  (return (LocalVariables|Getarray)))

(fn FillwithValueVectorBuffer
  (params (NewParam :type Array%20of%20Vectors) (NewParam1 :type Vector))
  (for _index (range 0 (- (Utilities|Array|Length NewParam) 1))
    (Utilities|Array|SetArrayElem NewParam _index NewParam1)))

(fn FillwithValueFloatBuffer
  (params (NewParam :type Array%20of%20Floats%20%28single-precision%29) (NewParam1 :type Float%20%28single-precision%29))
  (for _index (range 0 (- (Utilities|Array|Length NewParam) 1))
    (Utilities|Array|SetArrayElem NewParam _index NewParam1)))