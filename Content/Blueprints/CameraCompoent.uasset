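; Pawn camera component that smooths its yaw over recent direction samples while taking pitch and roll from control rotation.
; Each Update stores the yaw as a unit vector in a sample buffer and adjusts a running sum by the replaced entry, averaging angles without wraparound issues.
; It then fires a fan of nine debug-drawn visibility traces, whose results are unused.
; An older float-based averaging path remains disconnected.
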(event Custom|Update
  (params (direction :type Rotator))
  (bind _returnvalue (Class|KismetMathLibrary|CreateVectorfromYawPitch (.yaw direction) 0.0 1.0))
  (bind _owner (Variables|Default|Getowner))
  (bind _returnvalue_2 (Pawn|GetControlRotation _owner :!class /Script/Engine.Pawn))
  (bind _itemchanged (CallFunction|SetItemVectorBuffer (Variables|Default|GetvBuffer) (Variables|Default|GetcurrentSample) _returnvalue))
  (Math|Integer|IncrementInt (Variables|Default|GetcurrentSample)
    (:%20%20
      (bind _output_get (Variables|Default|Setaverage (+ (Variables|Default|Getaverage) (- _returnvalue _itemchanged))))
      (Transformation|SetRelativeRotation (Math|Rotator|MakeRotator (.roll _returnvalue_2) (.pitch _returnvalue_2) (.yaw (Math|Conversions|RotationFromXVector _output_get))) false false)
      (for _index (range -4 4)
        (Collision|LineTraceByChannel (Transformation|GetWorldLocation) (+ (Transformation|GetWorldLocation) (Math|Vector|RotateVector (Variables|Default|GettraceLength) (Math|Rotator|CombineRotators (Transformation|GetWorldRotation) (Math|Rotator|CombineRotators (* (Variables|Default|GetrotationStep) _index) "0,180.000000, 0")))) "TraceTypeQuery1" false 0 "ForOneFrame")))))

(event EventBeginPlay
  (bind _aspawn (Utilities|Casting|CastToPawn (Components|GetOwner)))
  (Variables|Default|Setowner _aspawn)
  (bind _buffer (CallFunction|CreateVectorBuffer (Variables|Default|GetnumberOfSamples)))
  (Variables|Default|SetvBuffer _buffer))